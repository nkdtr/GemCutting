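; BP_StoneCylinder is a gem-cutting stone Blueprint that supplies a cylinder as its base shape.
; CreateBaseShape uses Geometry Script's AppendCylinder to add the cylinder to the target mesh and returns the result, with radius, height, radial steps and origin driven by variables.
; The construction script only calls the parent, and the event graph holds only disabled stub events.
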(event EventBeginPlay
  (|CallParentFunction) ; This node is disabled and will not be called.\nDrag off pins to build functionality.
)

(event Collision|EventActorBeginOverlap
  (params (OtherActor :type Actor%20Object%20Reference))
  (|CallParentFunction OtherActor) ; This node is disabled and will not be called.\nDrag off pins to build functionality.
)

(event EventTick
  (params (DeltaSeconds :type Float%20%28single-precision%29))
  (|CallParentFunction DeltaSeconds) ; This node is disabled and will not be called.\nDrag off pins to build functionality.
)

(fn ConstructionScript
  (|CallParentFunction))

(fn CreateBaseShape
  (params (TargetMesh :type Dynamic%20Mesh%20Object%20Reference))
  (bind _returnvalue (GeometryScript|Primitives|AppendCylinder :TargetMesh TargetMesh :Radius (Variables|Default|GetRadius) :Height (Variables|Default|GetHeight) :RadialSteps (Variables|Default|GetRadial%20Steps) :Origin "Center" :Debug 0))
  (return _returnvalue))