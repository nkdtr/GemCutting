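; BP_CutterCone is a generated dynamic mesh actor that builds a faceted cone, named as a cutter for gem cutting.
; On mesh rebuild it appends a cone from Height, AngleDegree and RadialSteps, shifted down so the tip sits at the actor's origin.
; The base radius is divided by cos(π/RadialSteps), so the flat faces, rather than the corner edges, slope at exactly AngleDegree from horizontal.
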(event EventBeginPlay
  (|CallParentFunction) ; This node is disabled and will not be called.\nDrag off pins to build functionality.
)

(event Collision|EventActorBeginOverlap
  (params (OtherActor :type Actor%20Object%20Reference))
  (|CallParentFunction OtherActor) ; This node is disabled and will not be called.\nDrag off pins to build functionality.
)

(event EventTick
  (params (DeltaSeconds :type Float%20%28single-precision%29))
  (|CallParentFunction DeltaSeconds) ; This node is disabled and will not be called.\nDrag off pins to build functionality.
)

(event EventOnRebuildGeneratedMesh
  (params (TargetMesh :type Dynamic%20Mesh%20Object%20Reference))
  (bind _height (Variables|Default|GetHeight))
  (bind _radial_steps (Variables|Default|GetRadial%20Steps))
  (Class|GeometryScriptLibraryMeshPrimitiveFunctions|AppendCone :TargetMesh TargetMesh :Transform (Math|Conversions|ToTransform(Vector) (Math|Vector|MakeVector 0.0 0.0 (* _height -1.0))) :BaseRadius (Utilities|Operators|Divide _height (Math|Trig|Tan(Degrees) (Variables|Default|GetAngleDegree)) (Math|Trig|Cos(Radians) (Math|Float|MultiplybyPi (/ 1.0 (Math|Conversions|ToFloat(Integer) _radial_steps))))) :TopRadius 0.0 :Height _height :RadialSteps _radial_steps :HeightSteps 0 :Debug 0))

(fn ConstructionScript
  (|CallParentFunction))