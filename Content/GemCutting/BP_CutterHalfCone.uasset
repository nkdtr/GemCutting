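; Generated-mesh actor that builds a faceted half-cone cutter shape for gem cutting, using Geometry Script.
; On rebuild, it appends a box sized by Height and a radius derived from Height and AngleDegree.
; Plane cuts through the origin, tilted by AngleDegree about axes swept across 180 degrees in RadialSteps, carve the facets.
; A final simplify-to-planar pass cleans up the resulting mesh.
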(event EventBeginPlay
  (|CallParentFunction) ; This node is disabled and will not be called.\nDrag off pins to build functionality.
)

(event Collision|EventActorBeginOverlap
  (params (OtherActor :type Actor%20Object%20Reference))
  (|CallParentFunction OtherActor) ; This node is disabled and will not be called.\nDrag off pins to build functionality.
)

(event EventTick
  (params (DeltaSeconds :type Float%20%28single-precision%29))
  (|CallParentFunction DeltaSeconds) ; This node is disabled and will not be called.\nDrag off pins to build functionality.
)

(event EventOnRebuildGeneratedMesh
  (params (TargetMesh :type Dynamic%20Mesh%20Object%20Reference))
  (bind _radial_steps (Variables|Default|GetRadial%20Steps))
  (bind _returnvalue (CallFunction|CalcRadius))
  (bind _returnvalue_2 (Class|GeometryScriptLibraryMeshPrimitiveFunctions|AppendBox :TargetMesh TargetMesh :DimensionX (* _returnvalue 2.0) :DimensionY (* _returnvalue 2.0) :DimensionZ (Variables|Default|GetHeight) :Debug 0))
  (for _index (range 0 _radial_steps)
    (Class|GeometryScriptLibraryMeshBooleanFunctions|ApplyMeshPlaneCut :TargetMesh _returnvalue_2 :CutFrame (Math|Transform|MakeTransform "0, 0, 0" (Math|Vector|RotatorfromAxisandAngle (Math|Vector|MakeVector (Math|Trig|Cos(Degrees) (* (Math|Float|MakeLiteralFloat 1.8e+02) (/ _index _radial_steps))) (Math|Trig|Sin(Degrees) (* (Math|Float|MakeLiteralFloat 1.8e+02) (/ _index _radial_steps))) 0.0) (- 1.8e+02 (Variables|Default|GetAngleDegree)))) :Debug 0))
  (Class|GeometryScriptLibraryMeshSimplifyFunctions|ApplySimplifytoPlanar :TargetMesh _returnvalue_2 :Debug 0))

(fn ConstructionScript
  (|CallParentFunction))

(fn CalcRadius
  (return (/ (Variables|Default|GetHeight) (Math|Trig|Tan(Degrees) (Variables|Default|GetAngleDegree)))))