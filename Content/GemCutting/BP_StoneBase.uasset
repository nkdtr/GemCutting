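; BP_StoneBase is a generated dynamic mesh actor for gem cutting that builds a stone shaped by attached cutter actors.
; On rebuild, CreateBaseShape appends an eight-sided cylinder, which is optionally boolean-intersected with the mesh of each recursively attached BP_CutterBase.
; The result is then simplified to a tolerance using Geometry Script.
; CopyToStaticMesh bakes the dynamic mesh into the OutputMesh static mesh asset.
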(event EventBeginPlay)

(event Collision|EventActorBeginOverlap
  (params (OtherActor :type Actor%20Object%20Reference)))

(event EventTick
  (params (DeltaSeconds :type Float%20%28single-precision%29)))

(event Events|EventOnRebuildGeneratedMesh
  (params (TargetMesh :type Dynamic%20Mesh%20Object%20Reference))
  (Utilities|FlowControl|Sequence
    (:then_0
      (bind _returnvalue (CallFunction|CreateBaseShape TargetMesh))
      (Variables|Default|SetTarget%20Mesh _returnvalue))
    (:then_1
      (if (Variables|Default|GetbApplyCutters)
        (for _array_element (Actor|GetAttachedActors true true)
          (bind _asbp_cutter_base (Utilities|Casting|CastToBP_CutterBase _array_element))
          (bind _returnvalue_2 (DynamicMeshComponent|GetDynamicMesh (Variables|/Script/GeometryFramework.DynamicMeshActor|GetDynamicMeshComponent _asbp_cutter_base)))
          (Utilities|IsValid _returnvalue_2
            (:Is%20Valid
              (bind _returnvalue_3 (GeometryScript|Booleans|ApplyMeshBoolean :TargetMesh (Variables|Default|GetTarget%20Mesh) :TargetTransform (Transformation|GetWorldTransform (Variables|DynamicMeshActor|GetDynamicMeshComponent)) :ToolMesh _returnvalue_2 :ToolTransform (Transformation|GetWorldTransform (Variables|/Script/GeometryFramework.DynamicMeshActor|GetDynamicMeshComponent _asbp_cutter_base)) :Operation "Intersection" :Debug 0))
              (Variables|Default|SetTarget%20Mesh _returnvalue_3))))))
    (:then_2
      (Class|GeometryScriptLibraryMeshSimplifyFunctions|ApplySimplifytoTolerance :TargetMesh (Variables|Default|GetTarget%20Mesh) :Tolerance (Variables|Default|GetTolerance) :Debug 0))
    (:then_3
      (Variables|Default|SetTarget%20Mesh 0))))

(fn ConstructionScript)

(fn CopytoStaticMesh
  (bind _returnvalue (DynamicMeshComponent|GetDynamicMesh (Variables|DynamicMeshActor|GetDynamicMeshComponent)))
  (GeometryScript|StaticMesh|CopyMeshtoStaticMesh :FromDynamicMesh _returnvalue :ToStaticMeshAsset (Variables|Default|GetOutputMesh) :Debug 0))

(fn CreateBaseShape
  (params (TargetMesh :type Dynamic%20Mesh%20Object%20Reference))
  (bind _returnvalue (GeometryScript|Primitives|AppendCylinder :TargetMesh TargetMesh :RadialSteps 8 :Origin "Center" :Debug 0))
  (return _returnvalue))