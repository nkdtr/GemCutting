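; BP_CutterCylinder is a generated dynamic mesh actor that provides a cylinder shape, named as a cutter for gem cutting.
; On each mesh rebuild, Geometry Script appends a cylinder to the target mesh, sized by its Radius, Height and RadialSteps variables.
; It has no active runtime logic, and the file shows only the shape generation, with no cutting operation.
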(event EventBeginPlay
  (|CallParentFunction) ; This node is disabled and will not be called.\nDrag off pins to build functionality.
)

(event Collision|EventActorBeginOverlap
  (params (OtherActor :type Actor%20Object%20Reference))
  (|CallParentFunction OtherActor) ; This node is disabled and will not be called.\nDrag off pins to build functionality.
)

(event EventTick
  (params (DeltaSeconds :type Float%20%28single-precision%29))
  (|CallParentFunction DeltaSeconds) ; This node is disabled and will not be called.\nDrag off pins to build functionality.
)

(event EventOnRebuildGeneratedMesh
  (params (TargetMesh :type Dynamic%20Mesh%20Object%20Reference))
  (GeometryScript|Primitives|AppendCylinder :TargetMesh TargetMesh :Radius (Variables|Default|GetRadius) :Height (Variables|Default|GetHeight) :RadialSteps (Variables|Default|GetRadial%20Steps) :Debug 0))

(fn ConstructionScript
  (|CallParentFunction))